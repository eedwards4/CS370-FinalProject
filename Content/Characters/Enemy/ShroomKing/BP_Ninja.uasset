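; BP_Ninja is a side-scroller enemy that patrols back and forth along the Y axis and hurts the player on contact.
; Tick feeds constant movement input, flipping the Direction flag and actor yaw whenever velocity drops to zero.
; Capsule hits from BP_SideScrollerCharacter destroy the Ninja when the hit normal points steeply downward, as in a stomp.
; Other hits subtract LifePoints from the player, throttled by a DoOnce reset after a one-second delay.
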(event `self.ReceiveTick`
  (params (DeltaSeconds :type "Float (single-precision)"))
  (bind _returnvalue (== (`self.GetVelocity`) (0.0 0.0 0.0)))
  (if (`self.Direction`)
    (`self.AddMovementInput` (0.0 -1.0 0.0))
    (if _returnvalue
      (set `self.Direction` false)
      (`self.K2_SetActorRotation` (`KismetMathLibrary.MakeRotator` 0.0)))
    (else
      (`self.AddMovementInput` (0.0 1.0 0.0))
      (if _returnvalue
        (set `self.Direction` true)
        (`self.K2_SetActorRotation` (`KismetMathLibrary.MakeRotator` 0.0 0.0 -180.0))))))

(event `self.ReceiveBeginPlay`)

(event `self.CapsuleComponent.OnComponentHit`
  (params (HitComponent :type "PrimitiveComponent Object Reference") (OtherActor :type "Actor Object Reference") (OtherComp :type "PrimitiveComponent Object Reference") (NormalImpulse :type "Vector Structure") (Hit :type "HitResult Structure (by ref)"))
  (bind _asbp_side_scroller_character (cast `/Game/Characters/Player/BP_SideScrollerCharacter` OtherActor))
  (if (<= (.z (`.Normal` (`GameplayStatics.BreakHitResult` Hit))) -0.8)
    (`KismetSystemLibrary.PrintString` (`KismetStringLibrary.Conv_DoubleToString` (.z (`.Normal` (`GameplayStatics.BreakHitResult` Hit)))))
    (`self.K2_DestroyActor`)
    (else
      (`/Engine/EditorBlueprintResources/StandardMacros.DoOnce` false :!label _label
        (:`Completed`
          (set `/Game/Characters/Player/BP_SideScrollerCharacter.Life Points` (- (`/Game/Characters/Player/BP_SideScrollerCharacter.Life Points` _asbp_side_scroller_character) 5.0) _asbp_side_scroller_character)
          (`KismetSystemLibrary.Delay` 1.0)
          (goto _label :!via `Reset`))))))

(fn `UserConstructionScript`)