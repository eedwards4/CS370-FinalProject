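; Mushroom King enemy character for a side-scroller that patrols walk zones, hurts the player on contact and dies when stomped.
; Tick drives movement along the world Y axis while the overlapped actor implements the walk-zone interface, and leaving a zone flips direction and facing.
; Capsule hits on the player character use the hit normal to either destroy the enemy or subtract player Health, throttled by a DoOnce and Delay cooldown.
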(event `self.ReceiveTick`
  (params (DeltaSeconds :type "Float (single-precision)"))
  ;[1 1 1] Movement
  (if (`KismetSystemLibrary.DoesImplementInterface` (stale `self.CapsuleComponent.OnComponentBeginOverlap` OtherActor) "/Game/Characters/Enemy/Enemy_Walk_Zone/BP_WalkZone_Interface.BP_WalkZone_Interface_C")
    (if (`self.Direction`) :!label _label
      (`self.AddMovementInput` (0.0 -1.0 0.0))
      (`self.K2_SetActorRotation` (`KismetMathLibrary.MakeRotator` 0.0 0.0 -180.0))
      (else
        (`self.AddMovementInput` (0.0 1.0 0.0))
        (`self.K2_SetActorRotation` (`KismetMathLibrary.MakeRotator` 0.0))))))

(event `self.CapsuleComponent.OnComponentBeginOverlap`
  (params (OverlappedComponent :type "PrimitiveComponent Object Reference") (OtherActor :type "Actor Object Reference") (OtherComp :type "PrimitiveComponent Object Reference") (OtherBodyIndex :type Integer) (bFromSweep :type Boolean) (SweepResult :type "HitResult Structure (by ref)"))
  ;[1 1 1] Movement
)

(event `self.ReceiveActorEndOverlap`
  (params (OtherActor :type "Actor Object Reference"))
  ;[1 1 1] Movement
  (if (`KismetSystemLibrary.DoesImplementInterface` OtherActor "/Game/Characters/Enemy/Enemy_Walk_Zone/BP_WalkZone_Interface.BP_WalkZone_Interface_C")
    (set `self.Direction` (not (`self.Direction`)))
    (goto _label)))

(event `self.CapsuleComponent.OnComponentHit`
  (params (HitComponent :type "PrimitiveComponent Object Reference") (OtherActor :type "Actor Object Reference") (OtherComp :type "PrimitiveComponent Object Reference") (NormalImpulse :type "Vector Structure") (Hit :type "HitResult Structure (by ref)"))
  ;[1 1 1] Damange
  (bind _asbp_side_scroller_character (cast `/Game/Characters/Player/BP_SideScrollerCharacter` OtherActor))
  (if (<= (.z (`.Normal` (`GameplayStatics.BreakHitResult` Hit))) -0.8)
    (`self.K2_DestroyActor`)
    (else
      (`/Engine/EditorBlueprintResources/StandardMacros.DoOnce` false :!label _label_2
        (:`Completed`
          (set `/Game/Characters/Player/BP_SideScrollerCharacter.Health` (- (`/Game/Characters/Player/BP_SideScrollerCharacter.Health` _asbp_side_scroller_character) 5.0) _asbp_side_scroller_character)
          (`KismetSystemLibrary.Delay` 1.0)
          (goto _label_2 :!via `Reset`))))))

(fn `UserConstructionScript`)