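; SlipperySurface is a level-design Blueprint that makes the side-scroller character slide while inside its SlipCollision volume.
; On begin overlap, it casts to BP_SideScrollerCharacter, zeroes ground friction and lowers walking braking deceleration on its CharacterMovement.
; On end overlap, it writes back hard-coded normal values rather than restoring saved originals.
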(event `self.SlipCollision.OnComponentBeginOverlap`
  (params (OverlappedComponent :type "PrimitiveComponent Object Reference") (OtherActor :type "Actor Object Reference") (OtherComp :type "PrimitiveComponent Object Reference") (OtherBodyIndex :type Integer) (bFromSweep :type Boolean) (SweepResult :type "HitResult Structure (by ref)"))
  (if true
    (bind _asbp_side_scroller_character (cast `/Game/Characters/Player/BP_SideScrollerCharacter` OtherActor))
    (bind _charactermovement (`Character.CharacterMovement` _asbp_side_scroller_character))
    (set `CharacterMovementComponent.GroundFriction` 0.0 _charactermovement)
    (set `CharacterMovementComponent.BrakingDecelerationWalking` 350.0 _charactermovement)))

(event `self.SlipCollision.OnComponentEndOverlap`
  (params (OverlappedComponent :type "PrimitiveComponent Object Reference") (OtherActor :type "Actor Object Reference") (OtherComp :type "PrimitiveComponent Object Reference") (OtherBodyIndex :type Integer))
  (if true
    (bind _asbp_side_scroller_character (cast `/Game/Characters/Player/BP_SideScrollerCharacter` OtherActor))
    (bind _charactermovement (`Character.CharacterMovement` _asbp_side_scroller_character))
    (set `CharacterMovementComponent.GroundFriction` 8.0 _charactermovement)
    (set `CharacterMovementComponent.BrakingDecelerationWalking` 2000.0 _charactermovement)))

(fn `UserConstructionScript`)