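; Bouncepad is a level design actor that launches the player character straight up when they step onto it.
; The Pad component's begin-overlap event checks that the overlapping actor is the player pawn, then calls LaunchCharacter with a fixed, strong upward velocity that adds to existing motion.
; An Audio component plays on launch and is deactivated after a short delay.
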(event `self.pad.OnComponentBeginOverlap`
  (params (OverlappedComponent :type "PrimitiveComponent Object Reference") (OtherActor :type "Actor Object Reference") (OtherComp :type "PrimitiveComponent Object Reference") (OtherBodyIndex :type Integer) (bFromSweep :type Boolean) (SweepResult :type "HitResult Structure (by ref)"))
  (bind _returnvalue (`GameplayStatics.GetPlayerPawn` 0))
  (bind _audio (`self.Audio`))
  (`|ExecutionSequence`
    (:`then_0`
      (if (== OtherActor _returnvalue)
        (bind _ascharacter (cast `Character` _returnvalue))
        (`Character.LaunchCharacter` _ascharacter (0.0 0.0 3500.0) false false)
        (`|ExecutionSequence`
          (:`then_0`
            (`AudioComponent.Play` _audio 0.0)
            (`KismetSystemLibrary.Delay` 2.0)
            (`ActorComponent.Deactivate` _audio)))))))

(fn `UserConstructionScript`)